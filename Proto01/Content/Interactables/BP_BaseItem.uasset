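; BP_BaseItem is a base pickup item that an interacting instigator can collect into its inventory.
; On Interaction it checks the instigator for inventory space, passes ItemInfo through PickupMessage, then destroys itself.
; With no space, the item stays in place.
; The construction script stamps the actor's own class into ItemInfo while preserving the other fields, so each child class records itself automatically.
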(event EventInteraction
  (params (Instigator :type Player%20Character%20BP%20Object%20Reference))
  (if (Default|HasSpaceinInventory Instigator)
    (Class|BPIInteract|Pickup(Message) Instigator (Variables|Default|GetItemInfo))
    (Actor|DestroyActor)))

(fn ConstructionScript
  (Variables|Default|SetItemInfo (Utilities|Struct|MakeF_ItemInfo (.itemname (Variables|Default|GetItemInfo)) (.itemimage (Variables|Default|GetItemInfo)) (Utilities|GetClass self) (.itemindex (Variables|Default|GetItemInfo)) (.itemslot (Variables|Default|GetItemInfo))))
  (|CallParentFunction))